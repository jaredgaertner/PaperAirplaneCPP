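; Player-controlled paper airplane character that moves horizontally and vertically through axis inputs, using a sprite for its visual.
; MoveRight adds movement along world X and rotates the sprite between 0 and 180 degrees to match the input direction, leaving it unchanged at zero input.
; MoveUp drives flying by adding movement along the sprite's up vector, so that direction follows the sprite's orientation.
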(event `InputAxis|MoveRight`
  (params (AxisValue :type "Float (single-precision)"))
  (bind _sprite (`self.Sprite`))
  ;[1 1 1] Handle Movement and Rotation
  (if (> AxisValue 0.0)
    (`SceneComponent.K2_SetRelativeRotation` _sprite (struct) false false)
    (`self.AddMovementInput` (1.0 0.0 0.0) AxisValue :!label _label)
    (elif (< AxisValue 0.0)
      (`SceneComponent.K2_SetRelativeRotation` _sprite (struct :`Yaw` 180.0) false false)
      (goto _label))))

(event `InputAxis|MoveUp`
  (params (AxisValue :type "Float (single-precision)"))
  ;[1 1 1] Handle Movement and Rotation
  ;;[1 1 1] Handle Flying
  (`self.AddMovementInput` (`SceneComponent.GetUpVector` (`self.Sprite`)) AxisValue))

(fn `UserConstructionScript`)