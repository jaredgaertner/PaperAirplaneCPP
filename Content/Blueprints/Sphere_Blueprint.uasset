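; Sphere actor that the player can drag with the mouse along the world YZ plane.
; Hover, click and release events switch the cursor between grab hand, closed hand and default.
; Click and release open and close a Gate on Tick, which moves the actor to the Y and Z of a complex Visibility trace under the cursor, keeping its X, without sweep.
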(event `self.ReceiveActorBeginCursorOver`
  (set `PlayerController.CurrentMouseCursor` "GrabHand" (`GameplayStatics.GetPlayerController` 0)))

(event `self.ReceiveActorEndCursorOver`
  (set `PlayerController.CurrentMouseCursor` "Default" (`GameplayStatics.GetPlayerController` 0)))

(event `self.ReceiveTick`
  (params (DeltaSeconds :type "Float (single-precision)"))
  (`/Engine/EditorBlueprintResources/StandardMacros.Gate` true :!label _label
    (:`Exit`
      (`self.K2_SetActorLocation` (`KismetMathLibrary.MakeVector` (.x (`self.K2_GetActorLocation`)) (.y (`.Location` (`GameplayStatics.BreakHitResult` (`PlayerController.GetHitResultUnderCursorByChannel` (`GameplayStatics.GetPlayerController` 0) "TraceTypeQuery1" true)))) (.z (`.Location` (`GameplayStatics.BreakHitResult` (`PlayerController.GetHitResultUnderCursorByChannel` (`GameplayStatics.GetPlayerController` 0) "TraceTypeQuery1" true)))))))))

(event `self.ReceiveActorOnClicked`
  (set `PlayerController.CurrentMouseCursor` "GrabHandClosed" (`GameplayStatics.GetPlayerController` 0))
  (goto _label :!via `Open`))

(event `self.ReceiveActorOnReleased`
  (set `PlayerController.CurrentMouseCursor` "Default" (`GameplayStatics.GetPlayerController` 0))
  (goto _label :!via `Close`))

(fn `UserConstructionScript`)